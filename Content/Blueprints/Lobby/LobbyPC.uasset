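; Lobby player controller that represents each player in a multiplayer lobby and drives that player's lobby menu.
; Initial setup builds player info from the Steam name and avatar, then passes it to LobbyGM to swap the character and update everyone.
; Other events fill the menu's player list, map info and player count, or replace it with a loading screen.
; Being kicked opens the main menu, and both kick and EndPlay destroy the session.
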(event `InitialSetup`
  ;[1 1 1] Setup Initial stuff
  (bind _playerinfo (`self.SetupPlayerInfo`))
  (`self.CallUpdate` _playerinfo))

(event `CallUpdate`
  (params (PlayerInfo :type "/Game/Blueprints/AllLevels/PlayerInfo Structure") (ChangedStatus :type Boolean))
  (bind _aslobby_gm (cast `/Game/Blueprints/Lobby/LobbyGM` (`GameplayStatics.GetGameMode`) :!pure true))
  ;[1 1 1] Update GameMode info
  (bind _output_get (set `self.PlayerSettings` PlayerInfo))
  (`/Game/Blueprints/Lobby/LobbyGM.SwapCharacter` _aslobby_gm self (`.Characters_6_FA1ACDCE4A5421B8EAC737B4C6C5F50E` (break `/Game/Blueprints/AllLevels/PlayerInfo` _output_get)) ChangedStatus)
  (`/Game/Blueprints/Lobby/LobbyGM.EveryoneUpdate` _aslobby_gm))

(event `SetupLobbyMenu`
  (params (ServerName :type Text))
  ;[1 1 1] Create lobby menu widget
  (set `self.bShowMouseCursor` true)
  (bind _returnvalue (`|CreateWidget` "/Game/UI/Lobby/LobbyMenu.LobbyMenu_C" null ServerName))
  (bind _output_get (set `self.LobbyMenuWB` _returnvalue))
  (`UserWidget.AddToViewport` _output_get 0)
  (`WidgetBlueprintLibrary.SetInputMode_GameAndUIEx` self _output_get))

(event `AddPlayerInfo`
  (params (ConnectedPlayers :type "Array of /Game/Blueprints/AllLevels/PlayerInfo Structure"))
  (bind _lobbymenuwb (`self.LobbyMenuWB`))
  ;[1 1 1] Add Player to lobby menu
  (set `self.AllConnectedPlayers` ConnectedPlayers)
  (`/Engine/EditorBlueprintResources/StandardMacros.IsValid` _lobbymenuwb
    (:`Is Valid`
      (`/Game/UI/Lobby/LobbyMenu.ClearPlayerList` _lobbymenuwb)
      (for _array_element (`self.AllConnectedPlayers`)
        (`/Game/UI/Lobby/LobbyMenu.UpdatePlayerWindow` (`self.LobbyMenuWB`) _array_element)))))

(event `UpdateAvailableCharacters`
  (params (AvailableCharacters :type "Array of Boolean")))

(event `UpdateLobbySettings`
  (params (MapImage :type "Texture2D Object Reference") (MapName :type Text) (MapTime :type Text))
  (bind _lobbymenuwb (`self.LobbyMenuWB`))
  ;[1 1 1] Update lobby info
  (set `/Game/UI/Lobby/LobbyMenu.MapImage` MapImage _lobbymenuwb)
  (set `/Game/UI/Lobby/LobbyMenu.MapName` MapName _lobbymenuwb))

(event `ShowLoadingScreen`
  ;[1 1 1] Show Loading Screen
  (`Widget.RemoveFromParent` (`self.LobbyMenuWB`))
  (bind _returnvalue (`|CreateWidget` "/Game/UI/LoadingScreen.LoadingScreen_C" self))
  (`UserWidget.AddToViewport` _returnvalue 0))

(event `UpdateNumberOfPlayers`
  (params (CurrentPlayers :type Integer) (MaxPlayers :type Integer))
  (bind _lobbymenuwb (`self.LobbyMenuWB`))
  ;[1 1 1] Setup player count (current / max)
  (`/Engine/EditorBlueprintResources/StandardMacros.IsValid` _lobbymenuwb
    (:`Is Valid`
      (set `/Game/UI/Lobby/LobbyMenu.PlayersDisplay` (`|FormatText` "{Current} / {Max}" CurrentPlayers MaxPlayers) _lobbymenuwb))))

(event `self.ReceiveEndPlay`
  (params (EndPlayReason :type "EEndPlayReason Enum" :default "Destroyed"))
  ;[1 1 1] Called when disconnected or kicked
  (`DestroySessionCallbackProxy.DestroySession` self :!label _label))

(event `Kicked`
  ;[1 1 1] Called when disconnected or kicked
  (`GameplayStatics.OpenLevel` "MainMenu")
  (goto _label))

(fn `SetupPlayerInfo`
  (returns (PlayerInfo :type "/Game/Blueprints/AllLevels/PlayerInfo Structure"))
  (bind _uniquenetid (`AdvancedSessionsLibrary.GetUniqueNetID` self))
  (bind _returnvalue (`AdvancedSteamFriendsLibrary.GetSteamPersonaName` _uniquenetid))
  (bind _returnvalue_2 (`AdvancedSteamFriendsLibrary.GetSteamFriendAvatar` _uniquenetid)
    (:`OnSuccess`
      _)
    (:`OnFailure`
      _))
  (return (make `/Game/Blueprints/AllLevels/PlayerInfo` "Not Ready" "/Game/Characters/Base.Base_C" _returnvalue _returnvalue_2 "/Game/Mannequin/Character/Textures/UE4_Mannequin_MAT_MASKA.UE4_Mannequin_MAT_MASKA")))

(fn `UserConstructionScript`)