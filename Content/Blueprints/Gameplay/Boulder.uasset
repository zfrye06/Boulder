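; Boulder actor that tracks available spawn points and acts as a battlefield boundary for side-scroller characters.
; On BeginPlay it caches the Spawns actors overlapping KillZone into AvailableStarts.
; When a SideScrollerCharacterWithRep stops overlapping Box, it calls LeftBattlefield on that character's GameplayerPC.
; The matching EnteredBattlefield call and a spawn-list refresh are present but disconnected, so neither runs.
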(event `self.ReceiveBeginPlay`
  (for _array_element (`PrimitiveComponent.GetOverlappingActors` (`self.KillZone`) "/Game/Blueprints/Gameplay/Spawns.Spawns_C")
    (`KismetArrayLibrary.Array_Add` (`self.AvailableStarts`) (cast `/Game/Blueprints/Gameplay/Spawns` _array_element :!pure true)))
  (`KismetSystemLibrary.PrintString` "Added spawns"))

(event `self.ReceiveTick`
  (params (DeltaSeconds :type "Float (single-precision)")))

(event `self.Box.OnComponentEndOverlap`
  (params (OverlappedComponent :type "PrimitiveComponent Object Reference") (OtherActor :type "Actor Object Reference") (OtherComp :type "PrimitiveComponent Object Reference") (OtherBodyIndex :type Integer))
  (bind _asside_scroller_character_with_rep (cast `/Game/SideScrollerBP/Blueprints/SideScrollerCharacterWithRep` OtherActor))
  (bind _asgameplayer_pc (cast `/Game/Blueprints/Gameplay/GameplayerPC` (`Pawn.GetController` _asside_scroller_character_with_rep)))
  (`/Game/Blueprints/Gameplay/GameplayerPC.LeftBattlefield` _asgameplayer_pc))

(event `self.Box.OnComponentBeginOverlap`
  (params (OverlappedComponent :type "PrimitiveComponent Object Reference") (OtherActor :type "Actor Object Reference") (OtherComp :type "PrimitiveComponent Object Reference") (OtherBodyIndex :type Integer) (bFromSweep :type Boolean) (SweepResult :type "HitResult Structure (by ref)")))

(fn `UserConstructionScript`)