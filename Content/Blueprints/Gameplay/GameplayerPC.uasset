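; Player controller for gameplay matches in a multiplayer side-scroller, linking each player's pawn, widgets and the GameplayGM game mode.
; On begin play the local controller passes its character choice toward the server for spawning.
; Leaving the battlefield kills the pawn, possesses a Dead pawn at the Boulder and reports the death and last damage instigator.
; Other events drive countdown and death widgets, freezing, mesh glow, and the end screen before server travel to the lobby.
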(event `UpdateMaterial`
  (bind _asside_scroller_character_with_rep (cast `/Game/SideScrollerBP/Blueprints/SideScrollerCharacterWithRep` (`self.K2_GetPawn`)))
  (bind _mesh (`Character.Mesh` _asside_scroller_character_with_rep))
  (bind _returnvalue (`PrimitiveComponent.CreateDynamicMaterialInstance` _mesh 0 (`PrimitiveComponent.GetMaterial` _mesh 0)))
  (`MaterialInstanceDynamic.SetScalarParameterValue` _returnvalue "EmissiveStrength" 25.0))

(event `FreezePlayer`
  (bind _asside_scroller_character_with_rep (cast `/Game/SideScrollerBP/Blueprints/SideScrollerCharacterWithRep` (`self.K2_GetPawn` self)))
  (`/Game/SideScrollerBP/Blueprints/SideScrollerCharacterWithRep.SwitchState` _asside_scroller_character_with_rep "DONT MOVE"))

(event `EndGame`
  (`WidgetLayoutLibrary.RemoveAllWidgets`)
  (bind _returnvalue (`|CreateWidget` "/Game/UI/Gameplay/EndGame.EndGame_C" self))
  (`UserWidget.AddToViewport` _returnvalue 0)
  (bind _asside_scroller_character_with_rep (cast `/Game/SideScrollerBP/Blueprints/SideScrollerCharacterWithRep` (`self.K2_GetPawn` self)))
  (`/Game/SideScrollerBP/Blueprints/SideScrollerCharacterWithRep.SwitchState` _asside_scroller_character_with_rep "DONT MOVE")
  (`KismetSystemLibrary.Delay` 5.0)
  (`Widget.RemoveFromParent` _returnvalue)
  (`KismetSystemLibrary.ExecuteConsoleCommand` "servertravel /Game/Maps/Lobby" self))

(event `self.ReceiveBeginPlay`
  (`KismetSystemLibrary.ExecuteConsoleCommand` "r.MotionBlurQuality 0" self)
  (`KismetSystemLibrary.ExecuteConsoleCommand` "r.PostProcessAAQuality 2" self)
  (if (`self.IsLocalController`)
    (`WidgetLayoutLibrary.RemoveAllWidgets`)
    (`self.PassCharacterInfoToServer` (`self.PlayerSettings`))))

(event `PassCharacterInfoToServer`
  (params (PlayerInfo :type "/Game/Blueprints/AllLevels/PlayerInfo Structure"))
  (set `self.PlayerSettings` PlayerInfo)
  (bind _asgameplay_gm (cast `/Game/Blueprints/Gameplay/GameplayGM` (`GameplayStatics.GetGameMode`)))
  (`/Game/Blueprints/Gameplay/GameplayGM.InitialSpawn` _asgameplay_gm self (`.Characters_23_FA1ACDCE4A5421B8EAC737B4C6C5F50E` (break `/Game/Blueprints/AllLevels/PlayerInfo` (`self.PlayerSettings`)))))

(event `AddStartWidget`
  (bind _returnvalue (`|CreateWidget` "/Game/UI/Gameplay/Countdown.Countdown_C" self))
  (set `self.CountdownWB` _returnvalue)
  (`UserWidget.AddToViewport` (`self.CountdownWB`) 0))

(event `RemoveStartWidget`
  (`Widget.RemoveFromParent` (`self.CountdownWB`)))

(event `SetText`
  (params (Text :type Text))
  (set `/Game/UI/Gameplay/Countdown.Text` Text (`self.CountdownWB`)))

(event `LeftBattlefield`
  (params (LastDamageInstigator :type "/Game/Blueprints/Gameplay/GameplayerPC Object Reference"))
  (bind _returnvalue (`self.K2_GetPawn`))
  (bind _asside_scroller_character_with_rep (cast `/Game/SideScrollerBP/Blueprints/SideScrollerCharacterWithRep` _returnvalue))
  (`/Game/SideScrollerBP/Blueprints/SideScrollerCharacterWithRep.SwitchState` _asside_scroller_character_with_rep "die")
  (`KismetSystemLibrary.Delay` 2.0)
  (`self.K2_DestroyActor` _returnvalue)
  (bind _outactors (`GameplayStatics.GetAllActorsOfClass` "/Game/Blueprints/Gameplay/Boulder.Boulder_C"))
  (bind _returnvalue_2 (`|SpawnActorFromClass` "/Game/Blueprints/Gameplay/Dead.Dead_C" (`KismetMathLibrary.MakeTransform` (.location (`SceneComponent.K2_GetComponentToWorld` (`self.K2_GetRootComponent` (`|GetArrayItem` _outactors)))) (`KismetMathLibrary.MakeRotator` (.roll (.rotation (`SceneComponent.K2_GetComponentToWorld` (`self.K2_GetRootComponent` (`|GetArrayItem` _outactors))))) (.pitch (.rotation (`SceneComponent.K2_GetComponentToWorld` (`self.K2_GetRootComponent` (`|GetArrayItem` _outactors))))) 0.0) (.scale (`SceneComponent.K2_GetComponentToWorld` (`self.K2_GetRootComponent` (`|GetArrayItem` _outactors))))) "Undefined" "OverrideRootScale"))
  (`self.Possess` _returnvalue_2)
  (bind _asgameplay_gm (cast `/Game/Blueprints/Gameplay/GameplayGM` (`GameplayStatics.GetGameMode`)))
  (`/Game/Blueprints/Gameplay/GameplayGM.AddToDeadList` _asgameplay_gm self)
  (bind _asgameplay_gm_2 (cast `/Game/Blueprints/Gameplay/GameplayGM` (`GameplayStatics.GetGameMode`)))
  (`/Game/Blueprints/Gameplay/GameplayGM.GivePriority` _asgameplay_gm_2 LastDamageInstigator self))

(event `AddDeadWidget`
  (bind _returnvalue (`|CreateWidget` "/Game/UI/Gameplay/YouDied.YouDied_C" self))
  (`UserWidget.AddToViewport` _returnvalue 0))

(fn `UserConstructionScript`)