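; Barrel actor that continuously bobs up and down along the world Z axis.
; On BeginPlay it records the root's Z as the base height, then a timeline offsets the Barrel component from it by MaxRaise times the BarrelHeight track.
; The timeline loops as a ping-pong, reversing when it finishes at full height and otherwise playing again from the start.
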(event `self.ReceiveBeginPlay`
  (bind _barrel (`self.Barrel`))
  (set `self.BaseZ` (.z (`SceneComponent.K2_GetComponentLocation` (`self.DefaultSceneRoot`))))
  (bind (_direction _barrel_height) (`Timeline|Timeline_0` :`NewTime` 0.0 :!label _label)
    (:`Update`
      (`SceneComponent.K2_SetWorldLocation` _barrel (`KismetMathLibrary.MakeVector` (.x (`SceneComponent.K2_GetComponentLocation` _barrel)) (.y (`SceneComponent.K2_GetComponentLocation` _barrel)) (+ (* (`self.MaxRaise`) _barrel_height) (`self.BaseZ`))) false false))
    (:`Finished`
      (if (== _barrel_height 1.0)
        (goto _label :!via `Reverse`)
        (else
          (goto _label :!via `PlayFromStart`))))))

(fn `UserConstructionScript`)