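; Dashing state for a player state machine, giving a forced-length ground dash with dash dancing.
; On entry it zeroes velocity, turns the mesh to the dash direction and seeds a movement buffer.
; Each update feeds that stick-adjusted buffer into movement input until the timer ends in Running or Idle.
; Jump input, falling or an opposite stick smash exits early to JumpSquat, Jumping or a reversed Dashing.
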(event `/Game/Blueprints/States/State.Update`
  (params (dt :type "Float (single-precision)") (player :type "/Game/SideScrollerBP/Blueprints/SideScrollerCharacter Object Reference"))
  (bind _axis_move_right (`/Game/SideScrollerBP/Blueprints/SideScrollerCharacter.Axis Move Right` player))
  (bind _dash_direction_buffer (`self.Dash Direction Buffer`))
  (bind _returnvalue (* (`/Game/SideScrollerBP/Blueprints/SideScrollerCharacter.Axis Move Right` player) (`self.Dash Adjustment Strength`)))
  ;[1 1 1] Jump detection
  (if (`/Game/SideScrollerBP/Blueprints/SideScrollerCharacter.Button Jump` player)
    (`/Game/SideScrollerBP/Blueprints/SideScrollerCharacter.SwitchState` player "/Game/Blueprints/States/JumpSquat.JumpSquat_C")
    (else
      ;[1 1 1] Falling detection
      (if (`NavMovementComponent.IsFalling` (`Character.CharacterMovement` player))
        (`/Game/SideScrollerBP/Blueprints/SideScrollerCharacter.SwitchState` player "/Game/Blueprints/States/Jumping.Jumping_C")
        (else
          ;[1 1 1] dash dancing
          (if (`/Game/SideScrollerBP/Blueprints/SideScrollerCharacter.Stick Is Smashed` player)
            (if (>= (`KismetMathLibrary.Abs` (- _axis_move_right (`/Game/SideScrollerBP/Blueprints/SideScrollerCharacter.Dash Direction` player))) 1.2)
              (set `/Game/SideScrollerBP/Blueprints/SideScrollerCharacter.Dash Direction` (/ _axis_move_right (`KismetMathLibrary.Abs` _axis_move_right)) player)
              (`/Game/SideScrollerBP/Blueprints/SideScrollerCharacter.SwitchState` player "Dashing_C")
              (else
                ;[1 1 1] Dash adjustment
                (if (>= (`/Game/SideScrollerBP/Blueprints/SideScrollerCharacter.Dash Direction` player) 0.0) :!label _label
                  (set `self.Dash Direction Buffer` (- _dash_direction_buffer _returnvalue))
                  (else
                    (set `self.Dash Direction Buffer` (+ _dash_direction_buffer _returnvalue))))
                ;[1 1 1] Forced dash length
                (bind _output_get (set `self.Dash Length Timer` (+ (`self.Dash Length Timer`) dt)))
                (`Pawn.AddMovementInput` player (0.0 -1.0 0.0) (`self.Dash Direction Buffer`) false)
                (if (>= _output_get (`self.Dash Length`))
                  ;[1 1 1] forced dash over, return control to player.
                  (if (>= (`KismetMathLibrary.Abs` (`/Game/SideScrollerBP/Blueprints/SideScrollerCharacter.Axis Move Right` player)) 0.8)
                    (if (>= (`KismetMathLibrary.Abs` (- (`/Game/SideScrollerBP/Blueprints/SideScrollerCharacter.Axis Move Right` player) (`/Game/SideScrollerBP/Blueprints/SideScrollerCharacter.Dash Direction` player))) 1.2)
                      (`/Game/SideScrollerBP/Blueprints/SideScrollerCharacter.SwitchState` player "/Game/Blueprints/States/Idle.Idle_C" :!label _label_2)
                      (else
                        (`/Game/SideScrollerBP/Blueprints/SideScrollerCharacter.SwitchState` player "/Game/Blueprints/States/Running.Running_C")))
                    (else
                      (goto _label_2))))))
            (else
              (goto _label))))))))

(event `self.Initialize`
  (params (player :type "/Game/SideScrollerBP/Blueprints/SideScrollerCharacter Object Reference"))
  (bind _dash_direction (`/Game/SideScrollerBP/Blueprints/SideScrollerCharacter.Dash Direction` player))
  (set `self.Dash Direction Buffer` _dash_direction)
  (set `MovementComponent.Velocity` (0.0 0.0 0.0) (`Character.CharacterMovement` player))
  (`/Game/SideScrollerBP/Blueprints/SideScrollerCharacter.Set Mesh Rot` player (`KismetMathLibrary.MakeRotator` 0.0 0.0 (+ (* _dash_direction -90.0) -90.0))))

(event `self.CleanUp`
  (params (player :type "/Game/SideScrollerBP/Blueprints/SideScrollerCharacter Object Reference")))