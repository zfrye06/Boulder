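; Jump squat state for a player character: the short wind-up before a jump that decides between a short hop and a full hop.
; Update times how long jump is held, sets JumpZVelocity on release or at the time limit, and switches to Jumping, also doing so if the player starts falling.
; CleanUp calls Jump, adds velocity saved in Initialize, then applies stick-based influence to Y velocity, capped at JumpZVelocity.
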(event `/Game/Blueprints/States/State.Update`
  (params (dt :type "Float (single-precision)") (player :type "/Game/SideScrollerBP/Blueprints/SideScrollerCharacter Object Reference"))
  (bind _jump_squat_hold_timer (`self.Jump Squat Hold Timer`))
  (bind _charactermovement (`Character.CharacterMovement` player))
  (bind _returnvalue (>= _jump_squat_hold_timer (`self.Short Hop Time Limit`)))
  ;[1 1 1] Falling detection (You can slide off the map while jump squating.)
  (if (`NavMovementComponent.IsFalling` (`Character.CharacterMovement` player))
    (`/Game/SideScrollerBP/Blueprints/SideScrollerCharacter.SwitchState` player "/Game/Blueprints/States/Jumping.Jumping_C")
    (elif (or (not (`/Game/SideScrollerBP/Blueprints/SideScrollerCharacter.Button Jump` player)) _returnvalue)
      (if _returnvalue
        (set `CharacterMovementComponent.JumpZVelocity` (`self.Full Hop Z Vel`) _charactermovement)
        (else
          (set `CharacterMovementComponent.JumpZVelocity` (`self.Short Hop Z Vel`) _charactermovement)))
      (`/Game/SideScrollerBP/Blueprints/SideScrollerCharacter.SwitchState` player "/Game/Blueprints/States/Jumping.Jumping_C")
      (else
        (set `self.Jump Squat Hold Timer` (+ _jump_squat_hold_timer dt))))))

(event `self.Initialize`
  (params (player :type "/Game/SideScrollerBP/Blueprints/SideScrollerCharacter Object Reference"))
  (set `self.CurVelocity` (`MovementComponent.Velocity` (`Character.CharacterMovement` player))))

(event `self.CleanUp`
  (params (player :type "/Game/SideScrollerBP/Blueprints/SideScrollerCharacter Object Reference"))
  (bind _charactermovement (`Character.CharacterMovement` player))
  (bind _jumpzvelocity (`CharacterMovementComponent.JumpZVelocity` _charactermovement))
  (bind _x (.x (`MovementComponent.Velocity` _charactermovement)))
  (bind _z (.z (`MovementComponent.Velocity` _charactermovement)))
  (bind _returnvalue (- (.y (`MovementComponent.Velocity` _charactermovement)) (* (`/Game/SideScrollerBP/Blueprints/SideScrollerCharacter.Axis Move Right` player) (`self.Jump Direction Influence`))))
  (bind _returnvalue_2 (`KismetMathLibrary.Abs` _returnvalue))
  (`Character.Jump` player)
  ;[1 1 1] Velocity inheritance
  (set `MovementComponent.Velocity` (+ (`MovementComponent.Velocity` _charactermovement) (`self.CurVelocity`)) _charactermovement)
  ;[1 1 1] Jump Direction Influence
  (if (>= _returnvalue_2 _jumpzvelocity)
    (set `MovementComponent.Velocity` (`KismetMathLibrary.MakeVector` _x (* _jumpzvelocity (/ _returnvalue _returnvalue_2)) _z) _charactermovement)
    (else
      (set `MovementComponent.Velocity` (`KismetMathLibrary.MakeVector` _x _returnvalue _z) _charactermovement))))