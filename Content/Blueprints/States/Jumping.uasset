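; Jumping state for a player character, handling airborne fast fall, jump hold and release, sideways air control and wall jumps until landing returns it to Idle.
; After the stick has been neutral, a smashed stick opens a buffered wall jump attempt in that direction.
; A matching wall within the buffer turns the mesh, launches the jump and switches to WallJumpSquat.
; An expired attempt starts a cooldown before the next try.
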(event `/Game/Blueprints/States/State.Update`
  (params (dt :type "Float (single-precision)") (player :type "/Game/SideScrollerBP/Blueprints/SideScrollerCharacter Object Reference"))
  (bind _axis_move_right (`/Game/SideScrollerBP/Blueprints/SideScrollerCharacter.Axis Move Right` player))
  (bind _wall_jump_direction (`/Game/SideScrollerBP/Blueprints/SideScrollerCharacter.Wall Jump Direction` player))
  ;[1 1 1] fast fall
  (if (<= (`/Game/SideScrollerBP/Blueprints/SideScrollerCharacter.Axis Move Up` player) -0.8)
    (`/Game/SideScrollerBP/Blueprints/SideScrollerCharacter.FastFall` player))
  ;[1 1 1] landing detection
  (if (`NavMovementComponent.IsFalling` (`Character.CharacterMovement` player))
    (if (`/Game/SideScrollerBP/Blueprints/SideScrollerCharacter.Button Jump` player)
      (`Character.Jump` player)
      (else
        (`Character.StopJumping` player)))
    ;[1 1 1] air control
    (`Pawn.AddMovementInput` player (0.0 -1.0 0.0) (`/Game/SideScrollerBP/Blueprints/SideScrollerCharacter.Axis Move Right` player) false)
    (if (`self.BeenInNeutral`)
      ;[1 1 1] Actual wall jumping code, detects walls and if the attempted wall jump would work for it.
      (if (> (`self.AttemptingWallJump`) 0.0)
        (if (or (and (`/Game/SideScrollerBP/Blueprints/SideScrollerCharacter.CanWallJumpLeft` player) (== _wall_jump_direction -1.0)) (and (`/Game/SideScrollerBP/Blueprints/SideScrollerCharacter.CanWallJumpRight` player) (== _wall_jump_direction 1.0)))
          (`/Game/SideScrollerBP/Blueprints/SideScrollerCharacter.Set Mesh Rot` player (`KismetMathLibrary.MakeRotator` 0.0 0.0 (+ (* _wall_jump_direction -90.0) -90.0)))
          (`/Game/SideScrollerBP/Blueprints/SideScrollerCharacter.WallJump` player (`/Game/SideScrollerBP/Blueprints/SideScrollerCharacter.Wall Jump Direction` player))
          (`/Game/SideScrollerBP/Blueprints/SideScrollerCharacter.SwitchState` player "/Game/Blueprints/States/WallJumpSquat.WallJumpSquat_C")
          (else
            ;[1 1 1] Detects walljump attempts, and sets a timer and saves the direction of the attempt.
            (if (`/Game/SideScrollerBP/Blueprints/SideScrollerCharacter.Stick Is Smashed` player) :!label _label
              (if (and (<= (`self.WallJumpFailTimer`) 0.0) (<= (`self.AttemptingWallJump`) 0.0))
                (set `self.AttemptingWallJump` (`self.WallJumpBuffer`))
                (set `/Game/SideScrollerBP/Blueprints/SideScrollerCharacter.Wall Jump Direction` (/ _axis_move_right (`KismetMathLibrary.Abs` _axis_move_right)) player)))
            ;[1 1 1] Timer Decrements, increments. Detects if the player failed a wall jump and applies a cooldown.
            (if (> (`self.AttemptingWallJump`) 0.0)
              (set `self.AttemptingWallJump` (- (`self.AttemptingWallJump`) dt))
              (if (> (`self.AttemptingWallJump`) 0.0)
                (set `self.WallJumpFailTimer` (- (`self.WallJumpFailTimer`) dt) :!label _label_2)
                (else
                  (set `self.WallJumpFailTimer` 0.666)))
              (else
                (goto _label_2)))))
        (else
          (goto _label)))
      (else
        (set `self.BeenInNeutral` (`/Game/SideScrollerBP/Blueprints/SideScrollerCharacter.Stick Is Neutral` player))))
    (else
      (`/Game/SideScrollerBP/Blueprints/SideScrollerCharacter.SwitchState` player "/Game/Blueprints/States/Idle.Idle_C"))))