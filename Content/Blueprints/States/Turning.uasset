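; Turning state in the player's movement state machine, handling the skid when a dash changes direction.
; Initialize copies the player's DashDirection into a buffer, which Update eases toward zero each frame and feeds as movement input along the world Y axis.
; Jump input switches to JumpSquat and falling to Jumping.
; Once the buffer nears zero, DashDirection takes the sign of the horizontal input and the state switches to Dashing.
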(event `/Game/Blueprints/States/State.Update`
  (params (dt :type "Float (single-precision)") (player :type "/Game/SideScrollerBP/Blueprints/SideScrollerCharacter Object Reference"))
  (bind _axis_move_right (`/Game/SideScrollerBP/Blueprints/SideScrollerCharacter.Axis Move Right` player))
  ;[1 1 1] Jump Detection
  (if (`/Game/SideScrollerBP/Blueprints/SideScrollerCharacter.Button Jump` player)
    (`/Game/SideScrollerBP/Blueprints/SideScrollerCharacter.SwitchState` player "/Game/Blueprints/States/JumpSquat.JumpSquat_C")
    (else
      ;[1 1 1] Falling detection
      (if (`NavMovementComponent.IsFalling` (`Character.CharacterMovement` player))
        (`/Game/SideScrollerBP/Blueprints/SideScrollerCharacter.SwitchState` player "/Game/Blueprints/States/Jumping.Jumping_C")
        (else
          (bind _output_get (set `self.Dash Direction Buffer` (`|EaseFunction` "EaseOut" (* dt 6.5) (`self.Dash Direction Buffer`))))
          (`Pawn.AddMovementInput` player (0.0 -1.0 0.0) _output_get false)
          (if (<= (`KismetMathLibrary.Abs` _output_get) 0.05)
            (set `/Game/SideScrollerBP/Blueprints/SideScrollerCharacter.Dash Direction` (/ _axis_move_right (`KismetMathLibrary.Abs` _axis_move_right)) player)
            (`/Game/SideScrollerBP/Blueprints/SideScrollerCharacter.SwitchState` player "/Game/Blueprints/States/Dashing.Dashing_C")))))))

(event `self.Initialize`
  (params (player :type "/Game/SideScrollerBP/Blueprints/SideScrollerCharacter Object Reference"))
  (set `self.Dash Direction Buffer` (`/Game/SideScrollerBP/Blueprints/SideScrollerCharacter.Dash Direction` player)))