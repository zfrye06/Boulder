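; Player movement state for running, which drives the character along the world Y axis in its dash direction.
; Each Update checks in priority order, switching to JumpSquat on jump input or to Jumping when the character is falling.
; Otherwise it applies movement input, then switches to Idle on a neutral stick or to Turning when the stick axis strongly opposes the dash direction.
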(event `/Game/Blueprints/States/State.Update`
  (params (dt :type "Float (single-precision)") (player :type "/Game/SideScrollerBP/Blueprints/SideScrollerCharacter Object Reference"))
  (bind _dash_direction (`/Game/SideScrollerBP/Blueprints/SideScrollerCharacter.Dash Direction` player))
  ;[1 1 1] Jump Detection
  (if (`/Game/SideScrollerBP/Blueprints/SideScrollerCharacter.Button Jump` player)
    (`/Game/SideScrollerBP/Blueprints/SideScrollerCharacter.SwitchState` player "/Game/Blueprints/States/JumpSquat.JumpSquat_C")
    (else
      ;[1 1 1] Falling detection
      (if (`NavMovementComponent.IsFalling` (`Character.CharacterMovement` player))
        (`/Game/SideScrollerBP/Blueprints/SideScrollerCharacter.SwitchState` player "/Game/Blueprints/States/Jumping.Jumping_C")
        (else
          (`Pawn.AddMovementInput` player (0.0 -1.0 0.0) _dash_direction false)
          (if (`/Game/SideScrollerBP/Blueprints/SideScrollerCharacter.Stick Is Neutral` player)
            (`/Game/SideScrollerBP/Blueprints/SideScrollerCharacter.SwitchState` player "/Game/Blueprints/States/Idle.Idle_C")
            (elif (>= (`KismetMathLibrary.Abs` (- (`/Game/SideScrollerBP/Blueprints/SideScrollerCharacter.Axis Move Right` player) _dash_direction)) 1.5)
              (`/Game/SideScrollerBP/Blueprints/SideScrollerCharacter.SwitchState` player "/Game/Blueprints/States/Turning.Turning_C"))))))))