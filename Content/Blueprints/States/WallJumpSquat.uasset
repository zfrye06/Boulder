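; WallJumpSquat is a player state that adds a short wind-up before a wall jump.
; On entry it disables character movement and starts a countdown timer from the squat length.
; When the timer expires, it restores Falling movement, launches the player along the stored wall jump direction on Y with a vertical boost, keeping X velocity, then switches to the Jumping state.
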(event `/Game/Blueprints/States/State.Update`
  (params (dt :type "Float (single-precision)") (player :type "/Game/SideScrollerBP/Blueprints/SideScrollerCharacter Object Reference"))
  (bind _walljumpsquattimer (`self.WallJumpSquatTimer`))
  (bind _charactermovement (`Character.CharacterMovement` player))
  (if (<= _walljumpsquattimer 0.0)
    (`CharacterMovementComponent.SetMovementMode` (`Character.CharacterMovement` (stale `self.Initialize` player)) "MOVE_Falling" 0)
    (set `MovementComponent.Velocity` (`KismetMathLibrary.MakeVector` (.x (`MovementComponent.Velocity` _charactermovement)) (* (`/Game/SideScrollerBP/Blueprints/SideScrollerCharacter.Wall Jump Direction` player) (`self.WallJumpHorizontalStrength`)) (`self.WallJumpVerticalStrength`)) _charactermovement)
    (`/Game/SideScrollerBP/Blueprints/SideScrollerCharacter.SwitchState` player "/Game/Blueprints/States/Jumping.Jumping_C")
    (else
      (set `self.WallJumpSquatTimer` (- _walljumpsquattimer dt)))))

(event `self.Initialize`
  (params (player :type "/Game/SideScrollerBP/Blueprints/SideScrollerCharacter Object Reference"))
  (`CharacterMovementComponent.DisableMovement` (`Character.CharacterMovement` player))
  (set `self.WallJumpSquatTimer` (`self.WallJumpSquatLength`)))