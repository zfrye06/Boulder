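; Walking state in the player's state machine, handling ground movement along a single horizontal axis.
; Each Update switches to JumpSquat on jump input, Jumping when falling, or Idle when the move axis is zero.
; Otherwise it applies movement input along the world Y axis scaled by a walking multiplier and snaps the mesh yaw to face the direction of travel.
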(event `/Game/Blueprints/States/State.Update`
  (params (dt :type "Float (single-precision)") (player :type "/Game/SideScrollerBP/Blueprints/SideScrollerCharacter Object Reference"))
  (bind _axis_move_right (`/Game/SideScrollerBP/Blueprints/SideScrollerCharacter.Axis Move Right` player))
  ;[1 1 1] Jump Detection
  (if (`/Game/SideScrollerBP/Blueprints/SideScrollerCharacter.Button Jump` player)
    (`/Game/SideScrollerBP/Blueprints/SideScrollerCharacter.SwitchState` player "/Game/Blueprints/States/JumpSquat.JumpSquat_C")
    (else
      ;[1 1 1] Falling detection
      (if (`NavMovementComponent.IsFalling` (`Character.CharacterMovement` player))
        (`/Game/SideScrollerBP/Blueprints/SideScrollerCharacter.SwitchState` player "/Game/Blueprints/States/Jumping.Jumping_C")
        (else
          (`Pawn.AddMovementInput` player (0.0 -1.0 0.0) (* _axis_move_right (`self.Walking Multiplier`)) false)
          (if (== _axis_move_right 0.0)
            (`/Game/SideScrollerBP/Blueprints/SideScrollerCharacter.SwitchState` player "/Game/Blueprints/States/Idle.Idle_C")
            (else
              (`SceneComponent.K2_SetWorldRotation` (`Character.Mesh` player) (`KismetMathLibrary.MakeRotator` 0.0 0.0 (+ (* (/ _axis_move_right (`KismetMathLibrary.Abs` _axis_move_right)) -90.0) -90.0)) false false))))))))