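; MyInstance, apparently the game instance, manages the multiplayer front-end menus and online session entry.
; Show events lazily create and cache the main, server, host and lobby widgets, with the main and lobby menus also enabling the mouse cursor.
; LaunchLobby creates an Advanced Sessions session tagged with the server name, then opens Lobby as a listen server or returns to the main menu on failure.
; JoinGame joins a supplied session search result.
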(event `ShowLobbyMenu`
  ;[1 1 1] Show lobby menu
  (`/Engine/EditorBlueprintResources/StandardMacros.IsValid` (`self.LobbyMenu`)
    (:`Is Valid`
      _)
    (:`Is Not Valid`
      (bind _returnvalue (`|CreateWidget` "/Game/UI/Lobby/LobbyMenu.LobbyMenu_C" (`GameplayStatics.GetPlayerController` 0)))
      (set `self.LobbyMenu` _returnvalue)))
  (`UserWidget.AddToViewport` (`self.LobbyMenu`) 0)
  (set `PlayerController.bShowMouseCursor` true (`GameplayStatics.GetPlayerController` 0)))

(event `ShowMainMenu`
  ;[1 1 1] Show main menu
  (`/Engine/EditorBlueprintResources/StandardMacros.IsValid` (`self.MainMenu`)
    (:`Is Valid`
      _)
    (:`Is Not Valid`
      (bind _returnvalue (`|CreateWidget` "/Game/UI/MainMenu/MainMenu.MainMenu_C" (`GameplayStatics.GetPlayerController` 0)))
      (set `self.MainMenu` _returnvalue)))
  (`UserWidget.AddToViewport` (`self.MainMenu`) 0)
  (set `PlayerController.bShowMouseCursor` true (`GameplayStatics.GetPlayerController` 0)))

(event `ShowServerMenu`
  ;[1 1 1] Show server menu
  (`/Engine/EditorBlueprintResources/StandardMacros.IsValid` (`self.ServerMenu`)
    (:`Is Valid`
      _)
    (:`Is Not Valid`
      (bind _returnvalue (`|CreateWidget` "/Game/UI/MainMenu/ServerMenu.ServerMenu_C" (`GameplayStatics.GetPlayerController` 0)))
      (set `self.ServerMenu` _returnvalue)))
  (`UserWidget.AddToViewport` (`self.ServerMenu`) 0))

(event `ShowHostMenu`
  ;[1 1 1] Show host menu
  (`/Engine/EditorBlueprintResources/StandardMacros.IsValid` (`self.HostMenu`)
    (:`Is Valid`
      _)
    (:`Is Not Valid`
      (bind _returnvalue (`|CreateWidget` "/Game/UI/MainMenu/HostMenu.HostMenu_C" (`GameplayStatics.GetPlayerController` 0)))
      (set `self.HostMenu` _returnvalue)))
  (`UserWidget.AddToViewport` (`self.HostMenu`) 0))

(event `LaunchLobby`
  (params (`LAN?` :type Boolean) (ServerName :type Text) (MaxPlayers :type Integer))
  ;[1 1 1] Attempt to launch the lobby
  (`CreateSessionCallbackProxyAdvanced.CreateAdvancedSession` (`|MakeArray` (`AdvancedSessionsLibrary.MakeLiteralSessionPropertyString` "ServerName" (`KismetTextLibrary.Conv_TextToString` ServerName))) (`GameplayStatics.GetPlayerController` 0) MaxPlayers 0 `LAN?`
    (:`OnSuccess`
      (`GameplayStatics.OpenLevel` "Lobby" true "listen"))
    (:`OnFailure`
      (`KismetSystemLibrary.PrintString` "Failed")
      (`self.ShowMainMenu`))))

(event `JoinGame`
  (params (Session :type "BlueprintSessionResult Structure"))
  ;[1 1 1] Join game
  (`JoinSessionCallbackProxy.JoinSession` (`GameplayStatics.GetPlayerController` 0) Session))